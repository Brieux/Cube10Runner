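; Player pawn for an auto-runner: a physics mesh moves along Y at a boostable speed, and Space flips its gravity between floor and ceiling.
; Tick applies custom gravity, overrides Y velocity and shifts the spotlight hue.
; Space fires an impulse and locks flipping until ground or ceiling overlaps re-enable it and restart that side's Niagara effect.
; Death hides the mesh and plays a disintegration effect; camera-follow logic is disconnected.
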(event `self.ReceiveTick`
  (params (DeltaSeconds :type "Float (single-precision)"))
  (bind _staticmesh (`self.StaticMesh`))
  (bind _gravityvalue (`self.GravityValue`))
  ;[1 1 1] VelocityCompute
  (`self.FollowCamera`)
  (`PrimitiveComponent.AddForce` _staticmesh (`KismetMathLibrary.MakeVector` 0.0 0.0 (* (select `bool` (`self.InversedGravity?`) :`false` _gravityvalue :`true` (* _gravityvalue -1.0)) (`self.GravityMultiplier`))) "None" true)
  (bind _returnvalue (`PrimitiveComponent.GetPhysicsLinearVelocity` _staticmesh "None"))
  (`PrimitiveComponent.SetPhysicsLinearVelocity` _staticmesh (`KismetMathLibrary.MakeVector` (.x _returnvalue) (`self.AccelerationValue`) (.z _returnvalue)) false "None")
  (`self.ChangeColor`))

(event `Key|SpaceBar`
  (params (Key :type "Key Structure"))
  (bind _impulsevalue (`self.ImpulseValue`))
  ;[1 1 1] New
  (:`Pressed`
    (if (not (`self.Moving?`))
      (set `self.Moving?` true)
      (`ActorComponent.Deactivate` (`self.NiagaraCeil`))
      (`ActorComponent.Deactivate` (`self.NiagaraGround`))
      (bind _output_get (set `self.InversedGravity?` (not (`self.InversedGravity?`))))
      (`PrimitiveComponent.AddImpulse` (`self.StaticMesh`) (`KismetMathLibrary.MakeVector` 0.0 0.0 (* (select `bool` _output_get :`false` (* _impulsevalue -1.0) :`true` _impulsevalue) (`self.ImpulseMultiplier`))) "None" true))))

(event `self.GroundDetect.OnComponentBeginOverlap`
  (params (OverlappedComponent :type "PrimitiveComponent Object Reference") (OtherActor :type "Actor Object Reference") (OtherComp :type "PrimitiveComponent Object Reference") (OtherBodyIndex :type Integer) (bFromSweep :type Boolean) (SweepResult :type "HitResult Structure (by ref)"))
  ;[1 1 1] DetectGround and DetectCeil
  (set `self.Moving?` false)
  (`ActorComponent.Activate` (`self.NiagaraGround`) true))

(event `Boost`
  (params (BoostValue :type "Float (double-precision)"))
  ;[1 1 1] BoostSystem
  (set `self.AccelerationValue` (+ (`self.AccelerationValue`) BoostValue)))

(event `self.CeilDetect.OnComponentBeginOverlap`
  (params (OverlappedComponent :type "PrimitiveComponent Object Reference") (OtherActor :type "Actor Object Reference") (OtherComp :type "PrimitiveComponent Object Reference") (OtherBodyIndex :type Integer) (bFromSweep :type Boolean) (SweepResult :type "HitResult Structure (by ref)"))
  ;[1 1 1] DetectGround and DetectCeil
  (set `self.Moving?` false)
  (`ActorComponent.Activate` (`self.NiagaraCeil`) true))

(event `self.ReceiveBeginPlay`
  (bind (_relativelocation_x _relativelocation_y) (`KismetMathLibrary.BreakVector` (`SceneComponent.RelativeLocation` (`self.Camera`))))
  ;[1 1 1] CameraFollowSystem
  (set `self.OffsetCamera` _relativelocation_y)
  (`NiagaraComponent.SetPaused` (`self.NS_Desintégration`) true))

(event `FollowCamera`
  ;[1 1 1] CameraFollowSystem
)

(event `Death`
  (`NiagaraComponent.ResetSystem` (`self.NS_Desintégration`))
  (`NiagaraComponent.SetPaused` (`self.NS_Desintégration`) false)
  (`SceneComponent.SetVisibility` (`self.StaticMesh`) false false)
  (`SceneComponent.SetVisibility` (`self.NiagaraGround`) false false)
  (`SceneComponent.SetVisibility` (`self.NiagaraCeil`) false false))

(fn `ChangeColor`
  (bind _spotlight (`self.SpotLight`))
  (bind (_h _s _v _a) (`KismetMathLibrary.RGBToHSV` (`LightComponentBase.GetLightColor` _spotlight)))
  (`LightComponent.SetLightColor` _spotlight (`KismetMathLibrary.HSVToRGB` (+ _h 0.5) _s _v _a) true))

(fn `Move / Activate Niagara`
  (if (not (`self.Moving?`))
    _))

(fn `UserConstructionScript`)